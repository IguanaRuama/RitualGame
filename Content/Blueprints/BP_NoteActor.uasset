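; BP_NoteActor is a note actor, apparently for a rhythm game, that shows its active, hit or missed state through sphere colour.
; On BeginPlay it creates a dynamic material for the sphere and maps four directions (left, up, down, right) to spawn locations.
; Colour events set the NoteColour parameter to white, green or red.
; A MoveTimeline exists but is never run, so the file shows no movement.
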(event `self.ReceiveBeginPlay`
  (bind _returnvalue (`PrimitiveComponent.CreateDynamicMaterialInstance` (`self.Sphere`) 0 null "None"))
  (set `self.sphereDynamic` _returnvalue)
  (`self.setSpawnLocations`))

(event `setActiveColour`
  ;[0.6875 0.111 0.111 0.5] TEMP
  (`MaterialInstanceDynamic.SetVectorParameterValue` (`self.sphereDynamic`) "NoteColour" (`KismetMathLibrary.LinearColor_White`)))

(event `setHitColour`
  ;[0.6875 0.111 0.111 0.5] TEMP
  (`MaterialInstanceDynamic.SetVectorParameterValue` (`self.sphereDynamic`) "NoteColour" (`KismetMathLibrary.LinearColor_Green`)))

(event `setMissedColour`
  ;[0.6875 0.111 0.111 0.5] TEMP
  (`MaterialInstanceDynamic.SetVectorParameterValue` (`self.sphereDynamic`) "NoteColour" (`KismetMathLibrary.LinearColor_Red`)))

(fn `setSpawnLocations`
  (`BlueprintMapLibrary.Map_Add` (`self.spawnLocations`) "Left" (`self.spawnLocationLeft`))
  (`BlueprintMapLibrary.Map_Add` (`self.spawnLocations`) "Up" (`self.spawnLocationUp`))
  (`BlueprintMapLibrary.Map_Add` (`self.spawnLocations`) "Down" (`self.spawnLocationDown`))
  (`BlueprintMapLibrary.Map_Add` (`self.spawnLocations`) "Right" (`self.spawnLocationRight`)))

(fn `UserConstructionScript`)