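; BP_RhythmPlayer is the player Blueprint that captures directional note presses for a rhythm game.
; On BeginPlay it caches the game mode if it implements the NoteInputHandling interface.
; Each Left, Down, Up or Right press reads the current song time from the game mode and sends it back with the direction through interface messages, leaving note handling to the game mode.
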(event `self.ReceiveBeginPlay`
  (bind _returnvalue (`GameplayStatics.GetGameMode`))
  (if (`KismetSystemLibrary.DoesImplementInterface` _returnvalue "/Script/BardSim.NoteInputHandling")
    (set `self.gameMode` _returnvalue)))

(event `InputAction|Left`
  (params (Key :type "Key Structure"))
  (:`Pressed`
    (bind _returnvalue (message `NoteInputHandling.getSongTime` (`self.gameMode`)))
    (message `NoteInputHandling.handleNoteInput` (`self.gameMode`) "Left" _returnvalue)))

(event `InputAction|Down`
  (params (Key :type "Key Structure"))
  (:`Pressed`
    (bind _returnvalue (message `NoteInputHandling.getSongTime` (`self.gameMode`)))
    (message `NoteInputHandling.handleNoteInput` (`self.gameMode`) "Down" _returnvalue)))

(event `InputAction|Up`
  (params (Key :type "Key Structure"))
  (:`Pressed`
    (bind _returnvalue (message `NoteInputHandling.getSongTime` (`self.gameMode`)))
    (message `NoteInputHandling.handleNoteInput` (`self.gameMode`) "Up" _returnvalue)))

(event `InputAction|Right`
  (params (Key :type "Key Structure"))
  (:`Pressed`
    (bind _returnvalue (message `NoteInputHandling.getSongTime` (`self.gameMode`)))
    (message `NoteInputHandling.handleNoteInput` (`self.gameMode`) "Right" _returnvalue)))

(fn `UserConstructionScript`)