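; BP_Crowd is a crowd actor that moves to a requested location and rotation when its StartMove event is called.
; StartMove caches the current and target transforms, then plays a timeline whose Movement track lerps location and rotation without sweeping.
; On finish it snaps to the target location but restores the starting rotation, then prints a debug message.
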(event `self.startMove`
  (params (targetLocation :type "Vector Structure") (targetRotation :type "Rotator Structure"))
  (set `self.targetLocation` targetLocation)
  (set `self.targetRotation` targetRotation)
  (set `self.startLocation` (`self.K2_GetActorLocation` self))
  (set `self.startRotation` (`self.K2_GetActorRotation` self))
  (bind (_direction _movement) (`Timeline|Timeline` :!via `PlayFromStart`)
    (:`Update`
      (`self.K2_SetActorLocation` self (`KismetMathLibrary.VLerp` (`self.startLocation`) (`self.targetLocation`) _movement) false false)
      (`self.K2_SetActorRotation` self (`KismetMathLibrary.RLerp` (`self.startRotation`) (`self.targetRotation`) _movement) false))
    (:`Finished`
      (`self.K2_SetActorTransform` self (`KismetMathLibrary.MakeTransform` (`self.targetLocation`) (`self.startRotation`)) false false)
      (`KismetSystemLibrary.PrintString` "moved"))))

(fn `UserConstructionScript`)