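; Manager for a directional note-based music game that configures note spawning and pooling from song data.
; On BeginPlay it scans TargetPoints tagged Spawn, End or Pool to fill spawn and end location maps and the pool location.
; Each point's first tag supplies its Left, Up, Down or Right map key.
; UpdateSongData passes the note DataTable, BP_NoteActor class, speed and lead time to Initialise, then builds the pool.
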(event `self.ReceiveBeginPlay`
  (set `self.tempSpawnLocations` (`self.spawnLocations`))
  (set `self.tempEndLocations` (`self.endLocations`))
  (`self.setTargetPoints`))

(event `/Game/Blueprints/BPI_SongData.updateSongData`
  (params (dataTable :type "DataTable Object Reference") (leadTIme :type "Float (double-precision)") (speed :type "Float (double-precision)"))
  (`self.initialise` dataTable "/Game/Blueprints/BP_NoteActor.BP_NoteActor_C" speed leadTIme)
  (`self.initialisePool`))

(fn `setDirectionLocations`
  (params (Target :type "TargetPoint Object Reference") (Tags :type "Array of Name") (`Location Maps` :type "Map of ENoteDirection Enum to Actor Object Reference"))
  (returns (`Location Map` :type "Map of ENoteDirection Enum to Actor Object Reference"))
  (bind _output_get (set `self.directionTag` (`|GetArrayItem` Tags)))
  (switch `string` (`KismetStringLibrary.Conv_NameToString` _output_get)
    (:`Default`
      (`BlueprintMapLibrary.Map_Add` `Location Maps` "None" Target))
    (:`Left`
      (`BlueprintMapLibrary.Map_Add` `Location Maps` "Left" Target))
    (:`Up`
      (`BlueprintMapLibrary.Map_Add` `Location Maps` "Up" Target))
    (:`Down`
      (`BlueprintMapLibrary.Map_Add` `Location Maps` "Down" Target))
    (:`Right`
      (`BlueprintMapLibrary.Map_Add` `Location Maps` "Right" Target)))
  (return `Location Maps`))

(fn `setTargetPoints`
  (bind _outactors (`GameplayStatics.GetAllActorsOfClass` "/Script/Engine.TargetPoint"))
  (for _array_element _outactors
    (bind _tags (`Actor.Tags` _array_element))
    (if (`KismetArrayLibrary.Array_Contains` _tags "Spawn")
      (bind _location_map (`self.setDirectionLocations` _array_element _tags (`self.tempSpawnLocations`)))
      (set `self.spawnLocations` _location_map)
      (elif (`KismetArrayLibrary.Array_Contains` _tags "End")
        (bind _location_map_2 (`self.setDirectionLocations` _array_element _tags (`self.tempEndLocations`)))
        (set `self.endLocations` _location_map_2)
        (elif (`KismetArrayLibrary.Array_Contains` _tags "Pool")
          (bind _output_get (set `self.location` (`self.K2_GetActorLocation` _array_element)))
          (set `self.poolLocation` _output_get))))))

(fn `UserConstructionScript`)