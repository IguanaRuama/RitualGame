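; Rhythm game mode Blueprint that sets up and runs each song level and its UI.
; BeginPlay finds the camera, note spawner and crowd, loads song data by level name, derives note lead time from travel distance and speed, then starts the song.
; Scoring builds on parent logic and updates the overlay through an event.
; It also toggles pause and, at song end, shows any sheet-music unlock before the results screen.
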(event `self.ReceiveBeginPlay`
  (bind _returnvalue (`GameplayStatics.GetPlayerController` 0))
  (`self.setPlayerControllerCamera`)
  (`self.setSpawnManager`)
  (`self.setSongData`)
  (`self.setTravelDistance`)
  (`self.setCrowdPoints`)
  (message `/Game/Blueprints/BPI_SongData.updateSongData` (`self.noteSpawnManager`) (`self.currentSongDataTable`) (`self.leadTime`) (`self.noteSpeed`))
  ;[0.5628 1 0.0903 0.5] Overlay to Viewport
  (bind _returnvalue_2 (`|CreateWidget` "/Game/Widgets/WBP_Overlay.WBP_Overlay_C" _returnvalue))
  (set `self.overlayWidget` _returnvalue_2)
  (add `self.onScoreChanged` (delegate `updateOverlay`))
  (`UserWidget.AddToViewport` (`self.overlayWidget`) 0)
  (`WidgetBlueprintLibrary.SetInputMode_GameOnly` _returnvalue)
  (`self.startSong` 0.1))

(event `updateOverlay` :!signature `self.onScoreChanged`
  (params (newCombo :type Integer) (newScore :type Integer))
  ;[0.5628 1 0.0903 0.5] Overlay to Viewport
  (`/Game/Widgets/WBP_Overlay.onOverlayUpdate` (`self.overlayWidget`) (`KismetTextLibrary.Conv_IntToText` newScore) (`KismetTextLibrary.Conv_IntToText` newCombo)))

(event `self.handleNoteInput`
  (params (inputDirection :type "ENoteDirection Enum" :default "Left") (inputTime :type "Float (single-precision)"))
  (`parent.handleNoteInput` inputDirection inputTime)
  (`KismetSystemLibrary.PrintString` (`KismetStringLibrary.Conv_IntToString` (`self.score`))))

(event `self.onSongAudioFinished`
  (bind _returnvalue (`GameplayStatics.GetPlayerController` 0))
  (`parent.onSongAudioFinished`)
  (bind _returnvalue_2 (`self.wasSheetMusicUnlockedThisRound`))
  (if _returnvalue_2
    (bind _returnvalue_3 (`|CreateWidget` "/Game/Widgets/WBP_MusicScrapUnlock.WBP_MusicScrapUnlock_C" _returnvalue))
    (`UserWidget.AddToViewport` _returnvalue_3 0)
    (add `/Game/Widgets/WBP_MusicScrapUnlock.onUnlockDismissed` _returnvalue_3 (delegate `onUnlockDismissedHandler`))
    (bind _asbp_rhythm_game_instance (cast `/Game/Blueprints/BP_RhythmGameInstance` (`GameplayStatics.GetGameInstance`)))
    (bind _returnvalue_4 (`RhythmGameInstance.getCollectedSheetMusic` _asbp_rhythm_game_instance))
    (`/Game/Widgets/WBP_MusicScrapUnlock.playAppear` _returnvalue_3 (`KismetTextLibrary.Conv_IntToText` (`BlueprintSetLibrary.Set_Length` _returnvalue_4)) (`KismetTextLibrary.Conv_IntToText` (`KismetArrayLibrary.Array_Length` (`self.levelProgressionOrder`))))
    (else
      (bind _returnvalue_5 (`|CreateWidget` "/Game/Widgets/WBP_EndScreen.WBP_EndScreen_C" _returnvalue))
      (`UserWidget.AddToViewport` _returnvalue_5 0)
      (`self.setScoreUpdates` _returnvalue_5))))

(event `onUnlockDismissedHandler`
  ;[1 0.4869 0.6569 0.5] Binding Event for End Screen Show
  (bind _returnvalue (`|CreateWidget` "/Game/Widgets/WBP_EndScreen.WBP_EndScreen_C" (`GameplayStatics.GetPlayerController` 0)))
  (`UserWidget.AddToViewport` _returnvalue 0)
  (`self.setScoreUpdates` _returnvalue))

(event `self.togglePause`
  (bind _returnvalue (`GameplayStatics.GetPlayerController` 0))
  (bind _returnvalue_2 (`GameplayStatics.GetPlayerController` 0))
  ; Pause Logic
  (if (`GameplayStatics.IsGamePaused`)
    (`Widget.RemoveFromParent` (`self.pauseWidget`))
    (`GameplayStatics.SetGamePaused` false)
    (`self.unpauseTimers`)
    (`WidgetBlueprintLibrary.SetInputMode_GameOnly` _returnvalue_2)
    (set `PlayerController.bShowMouseCursor` false _returnvalue_2)
    (else
      (`GameplayStatics.SetGamePaused` true)
      (`self.pauseTimers`)
      (bind _returnvalue_3 (`|CreateWidget` "/Game/Widgets/WBP_Pause.WBP_Pause_C" _returnvalue))
      (bind _output_get (set `self.pauseWidget` _returnvalue_3))
      (`UserWidget.AddToViewport` _output_get 0)
      (`WidgetBlueprintLibrary.SetInputMode_GameAndUIEx` _returnvalue _output_get)
      (set `PlayerController.bShowMouseCursor` true _returnvalue))))

(fn `setCrowdPoints`
  (bind _outactors (`GameplayStatics.GetAllActorsOfClass` "/Game/Blueprints/BP_Crowd.BP_Crowd_C"))
  (set `self.spawnedCrowd` _outactors)
  (bind _outactors_2 (`GameplayStatics.GetAllActorsOfClassWithTag` "/Script/Engine.TargetPoint" "On"))
  (set `self.crowdOnscreenPoints` _outactors_2)
  (bind _outactors_3 (`GameplayStatics.GetAllActorsOfClassWithTag` "/Script/Engine.TargetPoint" "Off"))
  (set `self.crowdOffscreenPoints` _outactors_3)
  (for (_array_element _array_index) (`self.spawnedCrowd`)
    (bind _output (`|GetArrayItem` (`self.crowdOffscreenPoints`) _array_index))
    (`self.K2_SetActorLocation` _array_element (`self.K2_GetActorLocation` _output) false false)
    (`self.K2_SetActorRotation` _array_element (`self.K2_GetActorRotation` _output) false)))

(fn `setPassedText`
  (params (passed :type Boolean))
  (returns (passedText :type String))
  (if (== passed true)
    (set `self.passedText` "Passed")
    (else
      (bind _output_get (set `self.passedText` "Failed"))))
  (return _output_get))

(fn `setPlayerControllerCamera`
  (bind _outactors (`GameplayStatics.GetAllActorsOfClass` "/Script/Engine.CameraActor"))
  (set `self.cameraRef` (`|GetArrayItem` _outactors))
  (set `self.playerControllerRef` (`GameplayStatics.GetPlayerController` 0))
  (if (and (`KismetSystemLibrary.IsValid` (`self.cameraRef`)) (`KismetSystemLibrary.IsValid` (`self.playerControllerRef`)))
    (`PlayerController.SetViewTargetWithBlend` (`self.playerControllerRef`) (`self.cameraRef`) 0.0 "VTBlend_Linear" 0.0 false)))

(fn `setScoreUpdates`
  (params (widget :type "Object Object Reference"))
  (bind _passed (`self.passed`))
  (bind _passedtext (`self.setPassedText` _passed))
  (message `/Game/Blueprints/BPI_Scoring.updateScores` widget (`self.score`) (`self.grade`) (`self.perfectHits`) (`self.greatHits`) (`self.goodHits`) (`self.misses`) _passedtext _passed (`self.highestCombo`)))

(fn `setSongData`
  (bind _returnvalue (`GameplayStatics.GetCurrentLevelName` true))
  (bind _output_get (set `self.currentLevel` (`KismetStringLibrary.Conv_StringToName` _returnvalue)))
  (`self.loadSongForLevel` _output_get)
  (`self.initInstrumentAudioComponents`))

(fn `setSpawnManager`
  (bind _outactors (`GameplayStatics.GetAllActorsOfClass` "/Game/Blueprints/BP_NoteSpawnManager.BP_NoteSpawnManager_C"))
  (set `self.noteSpawnManager` (`|GetArrayItem` _outactors))
  (`KismetSystemLibrary.PrintString` (`KismetStringLibrary.Concat_StrStr` "NoteSpawnManager: " (`KismetStringLibrary.Conv_ObjectToString` (`self.noteSpawnManager`))) true true (struct :`R` 1.0 :`B` 0.827609 :`A` 1.0) 5.0))

(fn `setTravelDistance`
  (bind _returnvalue (`NoteSpawnManager.GetAverageNoteTravelDistance` (`self.noteSpawnManager`)))
  (set `self.noteTravelDistance` _returnvalue)
  (if (> (`self.noteSpeed`) 0.0)
    (set `self.leadTime` (/ (`self.noteTravelDistance`) (`self.noteSpeed`)))))

(fn `UserConstructionScript`)